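; BP_Camera is a camera Blueprint that spins a spring arm continuously around the world yaw axis at a set pitch.
; The construction script orients the arm to the CameraRotation pitch with zero yaw and roll.
; Each Tick adds DeltaSeconds plus SpeedRotation to the current yaw; because the two are summed rather than multiplied, spin speed depends on frame rate.
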(event `self.ReceiveTick`
  (params (DeltaSeconds :type "Float (single-precision)"))
  (bind _springarm (`self.SpringArm`))
  (`SceneComponent.K2_SetWorldRotation` _springarm (`KismetMathLibrary.MakeRotator` 0.0 (`self.Camera_Rotation`) (+ (+ DeltaSeconds (`self.Speed rotation`)) (.yaw (`SceneComponent.K2_GetComponentRotation` _springarm)))) false false))

(fn `UserConstructionScript`
  (locals (NewLocalVar :type "Rotator Structure" :default (struct)))
  (bind _camera_rotation (`self.Camera_Rotation`))
  (`SceneComponent.K2_SetWorldRotation` (`self.SpringArm`) (`KismetMathLibrary.MakeRotator` 0.0 _camera_rotation) false false)
  (set `self.Camera_Rotation` _camera_rotation))